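; Player controller that lets a client pay with a Nano cryptocurrency block to raise a wall on the server.
; OpenDoor passes the signed block and wall to a server event, which queries the account frontier and checks the sent amount and destination against the game instance's payment account.
; A valid block is submitted through the NanoManager, and its confirmation callback lifts the wall behind a DoOnce.
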(event `OpenDoor`
  (params (Block :type "Block Structure") (`Server wall` :type "/Game/Blueprints/ServerWall Object Reference"))
  ;[1 1 1] Executed on client, passing the block with required amount to open the wall
  (`self.OpenDoorEvent` Block `Server wall`))

(event `OpenDoorEvent`
  (params (Block :type "Block Structure") (Serverwall :type "/Game/Blueprints/ServerWall Object Reference"))
  ;[1 1 1] Executed on server, validates block and lifts the wall up if the correct amount in the block is sent
  (`KismetSystemLibrary.PrintString` "Call AccountFrontier")
  (`NanoManager.AccountFrontier` (`/Game/NanoGameInstance.NanoManager` (stale `self.ReceiveBeginPlay` _asnano_game_instance)) (delegate `OnAccountFrontier`) (`.account` (break `Block` Block))))

(event `OnPaymentMade`
  (params (data :type "ProcessResponseData Structure"))
  ;[1 1 1] Executed on server, validates block and lifts the wall up if the correct amount in the block is sent
  (if (`.error` (break `ProcessResponseData` data))
    (`KismetSystemLibrary.PrintString` "Error making payment")
    (else
      (`/Engine/EditorBlueprintResources/StandardMacros.DoOnce` false
        (:`Completed`
          (bind _rootcomponent (`Actor.RootComponent` (stale `OpenDoorEvent` Serverwall)))
          (`SceneComponent.K2_SetWorldLocation` _rootcomponent (+ (`SceneComponent.K2_GetComponentLocation` _rootcomponent) (0.0 0.0 750.0)) false false))))))

(event `OnAccountFrontier`
  (params (data :type "AccountFrontierResponseData Structure"))
  (bind (_account _hash _balance _representative _error) (break `AccountFrontierResponseData` data))
  ;[1 1 1] Executed on server, validates block and lifts the wall up if the correct amount in the block is sent
  (if _error
    (`KismetSystemLibrary.PrintString` "Account frontier failed")
    (else
      (bind (_account_2 _previous _representative_2 _balance_2 _link) (break `Block` (stale `OpenDoorEvent` Block)))
      (bind _returnvalue (`NanoBlueprintLibrary.Greater` _balance _balance_2))
      (if _returnvalue
        (bind _returnvalue_2 (`NanoBlueprintLibrary.Subtract` _balance _balance_2))
        (bind _returnvalue_3 (`NanoBlueprintLibrary.AccountFromPublicKey` _link))
        (if (`KismetStringLibrary.EqualEqual_StrStr` _returnvalue_2 "10")
          (if (`KismetStringLibrary.EqualEqual_StrStr` (`/Game/NanoGameInstance.PaymentAccount` (stale `self.ReceiveBeginPlay` _asnano_game_instance)) _returnvalue_3)
            (`KismetSystemLibrary.PrintString` "Wait confirmation")
            (`NanoManager.SendWaitConfirmationBlock` (`/Game/NanoGameInstance.NanoManager` (stale `self.ReceiveBeginPlay` _asnano_game_instance)) (delegate `OnPaymentMade`) (stale `OpenDoorEvent` Block))
            (else
              (`KismetSystemLibrary.PrintString` "Accounts do not match")))
          (else
            (`KismetSystemLibrary.PrintString` "Amounts do not match!!")))))))

(event `self.ReceiveBeginPlay`
  ;[1 1 1] Executed on server, validates block and lifts the wall up if the correct amount in the block is sent
  (`/Engine/EditorBlueprintResources/ActorMacros.Switch Has Authority`
    (:`Authority`
      (bind _asnano_game_instance (cast `/Game/NanoGameInstance` (`GameplayStatics.GetGameInstance`))))))

(fn `UserConstructionScript`)