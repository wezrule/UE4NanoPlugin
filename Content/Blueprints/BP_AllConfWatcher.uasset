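; Trigger button actor that toggles listening to all Nano websocket confirmations and shows the latest one.
; Begin and end overlap share a FlipFlop that turns the button's dynamic material green or red via a scalar parameter.
; A nested FlipFlop on the green branch alternates between ListenAll with response binding and UnlistenAll with unbinding, using the game instance's websocket.
; Each response writes transaction and block details to the RoomDescription's LastConfirmation text.
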(event `self.Trigger collision.OnComponentBeginOverlap`
  (params (OverlappedComponent :type "PrimitiveComponent Object Reference") (OtherActor :type "Actor Object Reference") (OtherComp :type "PrimitiveComponent Object Reference") (OtherBodyIndex :type Integer) (bFromSweep :type Boolean) (SweepResult :type "HitResult Structure (by ref)"))
  (bind _button_light_material (`self.Button light material`))
  (`/Engine/EditorBlueprintResources/StandardMacros.FlipFlop` :!label _label
    (:`A`
      (`MaterialInstanceDynamic.SetScalarParameterValue` _button_light_material "State" 1.0) ; Change a scalar value in the button material that turns it green
      (`/Engine/EditorBlueprintResources/StandardMacros.FlipFlop`
        (:`A`
          (bind _nanowebsocket (`/Game/NanoGameInstance.NanoWebsocket` (stale `self.ReceiveBeginPlay` _asnano_game_instance)))
          (`NanoWebsocket.ListenAll` _nanowebsocket)
          ;[1 1 1] This hooks into listening to all websocket events
          (add `NanoWebsocket.onResponse` _nanowebsocket (delegate `OnConfirmationResponse`)))
        (:`B`
          (`NanoWebsocket.UnlistenAll` _nanowebsocket)
          (remove `NanoWebsocket.onResponse` _nanowebsocket (delegate `OnConfirmationResponse`)))))
    (:`B`
      (`MaterialInstanceDynamic.SetScalarParameterValue` _button_light_material "State" 0.0) ; Change a scalar value in the button material that turns it back to red
    )))

(event `self.Trigger collision.OnComponentEndOverlap`
  (params (OverlappedComponent :type "PrimitiveComponent Object Reference") (OtherActor :type "Actor Object Reference") (OtherComp :type "PrimitiveComponent Object Reference") (OtherBodyIndex :type Integer))
  (goto _label))

(event `self.ReceiveBeginPlay`
  (bind _asnano_game_instance (cast `/Game/NanoGameInstance` (`GameplayStatics.GetGameInstance`))))

(event `OnConfirmationResponse`
  (params (data :type "WebsocketConfirmationResponseData Structure (by ref)") (websocket :type "NanoWebsocket Object Reference"))
  (bind (_account _amount _hash _block) (break `WebsocketConfirmationResponseData` data))
  (bind (_account_2 _previous _representative _balance _link _subtype _work) (break `WebsocketBlock` _block))
  (`TextRenderComponent.K2_SetText` (`/Game/Blueprints/ListenAllConfs.Last confirmation` (`self.RoomDescription`)) (`KismetTextLibrary.Conv_StringToText` (`KismetStringLibrary.Concat_StrStr` (`KismetStringLibrary.Concat_StrStr` "Account: " _account "<br>" "Amount: " _amount "<br>" "Hash: " _hash "<br><br>") "Block: " "<br>" "Account: " _account_2 "<br>" "Previous: " _previous "<br>" "Representative: " _representative "<br>" "Balance: " _balance "<br>" "Link: " _link "<br>" "Subtype: " (`|GetEnumeratorNameAsString` _subtype) "<br>" "Work: " _work "<br>"))))

(fn `UserConstructionScript`
  (bind _returnvalue (`PrimitiveComponent.CreateDynamicMaterialInstance` (`self.ButtonMesh`) 2 null "None"))
  (set `self.Button light material` _returnvalue) ; Save a reference to the Dynamic Material Instance for use in the event graph
)