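; Arcade button actor that shows a Nano cryptocurrency payment QR code while a pawn stands in its trigger.
; Begin and end overlap share a FlipFlop that toggles the button's light material and the QR widget.
; The QR encodes a seed-derived account and random amount, watched over websocket with a single-use payment listener.
; On payment it removes the widget, requests receipt of the block, increments the seed index and unwatches.
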(event `self.Trigger collision.OnComponentBeginOverlap`
  (params (OverlappedComponent :type "PrimitiveComponent Object Reference") (OtherActor :type "Actor Object Reference") (OtherComp :type "PrimitiveComponent Object Reference") (OtherBodyIndex :type Integer) (bFromSweep :type Boolean) (SweepResult :type "HitResult Structure (by ref)"))
  (bind _button_light_material (`self.Button light material`))
  (`/Engine/EditorBlueprintResources/StandardMacros.FlipFlop` :!label _label
    (:`A`
      (`MaterialInstanceDynamic.SetScalarParameterValue` _button_light_material "State" 1.0) ; Change a scalar value in the button material that turns it green
      ;[1 1 1] Create and show the QR Code
      (bind _returnvalue (`|CreateWidget` "/Nano/QRCodePlane.QRCodePlane_C"))
      (bind _account (`/Game/NanoGameInstance.Account` (stale `self.ReceiveBeginPlay` _asnano_game_instance)))
      (if (`KismetStringLibrary.NotEqual_StrStr` _account)
        (bind _output_get (set `self.AmountListeningFor` (`KismetStringLibrary.Conv_IntToString` (`KismetMathLibrary.RandomInteger` 100))))
        (bind _returnvalue_2 (`NanoBlueprintLibrary.AccountFromSeed` (`/Game/NanoGameInstance.Seed` (stale `self.ReceiveBeginPlay` _asnano_game_instance)) (`self.seedIndex`)))
        (bind _qrcodeimage (`/Nano/QRCodePlane.QRCodeImage` _returnvalue))
        (bind _returnvalue_3 (`NanoBlueprintLibrary.GenerateQRCodeTextureWithAmount` (`KismetMathLibrary.FTrunc` (`KismetMathLibrary.BreakVector2D` (`CanvasPanelSlot.GetSize` (`WidgetLayoutLibrary.SlotAsCanvasSlot` _qrcodeimage)))) _returnvalue_2 _output_get))
        (`Image.SetBrushFromTexture` _qrcodeimage _returnvalue_3 false)
        ;[1 1 1] Listen for payment of this amount to this account (must be watching this account).
        ; This approach is only recommended for 1 off payments, and only 1 can be active at a time. It relies on pending blocks so make no other wallets are pocketing these funds at same time
        (`UserWidget.AddToViewport` _returnvalue 0)
        (bind _nanomanager (`/Game/NanoGameInstance.NanoManager` (stale `self.ReceiveBeginPlay` _asnano_game_instance)))
        (bind _nanowebsocket (`/Game/NanoGameInstance.NanoWebsocket` (stale `self.ReceiveBeginPlay` _asnano_game_instance)))
        (bind _returnvalue_4 (`NanoManager.Watch` :`self` _nanomanager :`account` _returnvalue_2 :`websocket` _nanowebsocket))
        (bind _output_get_2 (set `self.watcherId` _returnvalue_4))
        (`NanoManager.SingleUseAccountListenForPaymentWaitConfirmation` _nanomanager (delegate `OnPayment`) _returnvalue_2 (`self.AmountListeningFor`))
        (else
          (`KismetSystemLibrary.PrintString` "Have not created a seed yet!"))))
    (:`B`
      (`MaterialInstanceDynamic.SetScalarParameterValue` _button_light_material "State" 0.0) ; Change a scalar value in the button material that turns it back to red
      (`Widget.RemoveFromParent` _returnvalue)
      (`NanoManager.Unwatch` _nanomanager _account (`self.watcherId`) _nanowebsocket))))

(event `OnPayment`
  (params (hash :type String))
  ;[1 1 1] Listen for payment of this amount to this account (must be watching this account).
  ; This approach is only recommended for 1 off payments, and only 1 can be active at a time. It relies on pending blocks so make no other wallets are pocketing these funds at same time
  (`KismetSystemLibrary.PrintString` "Payment made!")
  (`Widget.RemoveFromParent` (stale `self.Trigger collision.OnComponentBeginOverlap` _returnvalue))
  (bind _returnvalue (`NanoBlueprintLibrary.PrivateKeyFromSeed` (`/Game/NanoGameInstance.Seed` (stale `self.ReceiveBeginPlay` _asnano_game_instance))))
  (bind _nanomanager (`/Game/NanoGameInstance.NanoManager` (stale `self.ReceiveBeginPlay` _asnano_game_instance)))
  ;;[1 1 1] Don't care too much about ths outcome, can always be reconsolidated later if necessary
  (`NanoManager.Receive` _nanomanager (delegate `OnReceive`) _returnvalue hash (`self.AmountListeningFor`))
  (`/Engine/EditorBlueprintResources/StandardMacros.IncrementInt` (`self.seedIndex`)
    (:`  `
      (`NanoManager.Unwatch` _nanomanager (stale `self.Trigger collision.OnComponentBeginOverlap` _returnvalue_2) (stale `self.Trigger collision.OnComponentBeginOverlap` _output_get_2) (`/Game/NanoGameInstance.NanoWebsocket` (stale `self.ReceiveBeginPlay` _asnano_game_instance))))))

(event `self.Trigger collision.OnComponentEndOverlap`
  (params (OverlappedComponent :type "PrimitiveComponent Object Reference") (OtherActor :type "Actor Object Reference") (OtherComp :type "PrimitiveComponent Object Reference") (OtherBodyIndex :type Integer))
  (goto _label))

(event `OnReceive`
  (params (data :type "ProcessResponseData Structure"))
  ;[1 1 1] Listen for payment of this amount to this account (must be watching this account).
  ; This approach is only recommended for 1 off payments, and only 1 can be active at a time. It relies on pending blocks so make no other wallets are pocketing these funds at same time
  (if (`.error` (break `ProcessResponseData` data))
    (`KismetSystemLibrary.PrintString` "Error arcade pocketing block")))

(event `self.ReceiveBeginPlay`
  (bind _asnano_game_instance (cast `/Game/NanoGameInstance` (`GameplayStatics.GetGameInstance`))))

(fn `UserConstructionScript`
  (bind _returnvalue (`PrimitiveComponent.CreateDynamicMaterialInstance` (`self.ButtonMesh`) 2 null "None"))
  (set `self.Button light material` _returnvalue) ; Save a reference to the Dynamic Material Instance for use in the event graph
)