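; Arcade payout trigger that shows a QR code of a Nano private key so the player can withdraw funds.
; Begin and end overlap share a FlipFlop toggling the button light and QR widget.
; The key derives from the game seed and room's seed index; its QR appears only if the wallet balance is positive.
; NanoManager then awaits payout or expiry to remove the widget; toggling off while visible cancels listening.
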(event `self.Trigger collision.OnComponentBeginOverlap`
  (params (OverlappedComponent :type "PrimitiveComponent Object Reference") (OtherActor :type "Actor Object Reference") (OtherComp :type "PrimitiveComponent Object Reference") (OtherBodyIndex :type Integer) (bFromSweep :type Boolean) (SweepResult :type "HitResult Structure (by ref)"))
  (bind _button_light_material (`self.Button light material`))
  (`/Engine/EditorBlueprintResources/StandardMacros.FlipFlop` :!label _label
    (:`A`
      (`MaterialInstanceDynamic.SetScalarParameterValue` _button_light_material "State" 1.0) ; Change a scalar value in the button material that turns it green
      (if (!= (`/Game/Blueprints/ArcadeQRCode.seedIndex` (`self.RoomDescription`)) 0)
        ;[1 1 1] Create and show the QR Code
        (bind _returnvalue (`|CreateWidget` "/Nano/QRCodePlane.QRCodePlane_C"))
        (if (`KismetStringLibrary.NotEqual_StrStr` (`/Game/NanoGameInstance.Account` (stale `self.ReceiveBeginPlay` _asnano_game_instance)))
          (bind _seed (`/Game/NanoGameInstance.Seed` (stale `self.ReceiveBeginPlay` _asnano_game_instance)))
          (bind _returnvalue_2 (`NanoBlueprintLibrary.PrivateKeyFromSeed` _seed (`/Game/Blueprints/ArcadeQRCode.seedIndex` (`self.RoomDescription`))))
          (bind _returnvalue_3 (`NanoBlueprintLibrary.AccountFromPrivateKey` _returnvalue_2))
          (bind _nanomanager (`/Game/NanoGameInstance.NanoManager` (stale `self.ReceiveBeginPlay` _asnano_game_instance)))
          (`NanoManager.GetWalletBalance` _nanomanager (delegate `OnWalletBalance`) _returnvalue_3)
          (else
            (`KismetSystemLibrary.PrintString` "No seed detected")))
        (else
          (`KismetSystemLibrary.PrintString` "Haven't paid to play yet!"))))
    (:`B`
      (`MaterialInstanceDynamic.SetScalarParameterValue` _button_light_material "State" 0.0) ; Change a scalar value in the button material that turns it back to red
      (if (`Widget.IsInViewport` _returnvalue)
        (`Widget.RemoveFromParent` _returnvalue)
        ;[1 1 1] If the user moves away the payment can still be receive, so this ensures the event won't be called
        (if (`KismetStringLibrary.NotEqual_StrStr` "" _seed)
          (bind _returnvalue_4 (`NanoBlueprintLibrary.AccountFromSeed` _seed (`/Game/Blueprints/ArcadeQRCode.seedIndex` (`self.RoomDescription`))))
          (`NanoManager.CancelPayout` _nanomanager _returnvalue_4 (`/Game/NanoGameInstance.NanoWebsocket` (stale `self.ReceiveBeginPlay` _asnano_game_instance))))))))

(event `OnWalletDrained`
  (params (expired :type Boolean))
  ;[1 1 1] Listens for a send from the payout account. This is not guarenteed to happen, so have a timeout or something to go to the next screen.
  (if expired
    (`KismetSystemLibrary.PrintString` "Timer expired")
    (else
      (`KismetSystemLibrary.PrintString` "Private key paid out!")))
  (`Widget.RemoveFromParent` (stale `self.Trigger collision.OnComponentBeginOverlap` _returnvalue)))

(event `self.Trigger collision.OnComponentEndOverlap`
  (params (OverlappedComponent :type "PrimitiveComponent Object Reference") (OtherActor :type "Actor Object Reference") (OtherComp :type "PrimitiveComponent Object Reference") (OtherBodyIndex :type Integer))
  (goto _label))

(event `OnWalletBalance`
  (params (data :type "GetBalanceResponseData Structure"))
  (bind (_account _balance _pending _error) (break `GetBalanceResponseData` data))
  (bind _expirytime (`self.expiryTime`))
  ;[1 1 1] Create and show the QR Code
  (if _error
    (`KismetSystemLibrary.PrintString` "Error getting wallet balance for payment qr code")
    (else
      (bind _returnvalue (`NanoBlueprintLibrary.Greater` _balance "0"))
      (if _returnvalue
        (bind _qrcodeimage (`/Nano/QRCodePlane.QRCodeImage` (stale `self.Trigger collision.OnComponentBeginOverlap` _returnvalue)))
        (bind _returnvalue_2 (`NanoBlueprintLibrary.GenerateQRCodeTextureWithPrivateKey` (`KismetMathLibrary.FTrunc` (`KismetMathLibrary.BreakVector2D` (`CanvasPanelSlot.GetSize` (`WidgetLayoutLibrary.SlotAsCanvasSlot` _qrcodeimage)))) (stale `self.Trigger collision.OnComponentBeginOverlap` _returnvalue_2)))
        (`Image.SetBrushFromTexture` _qrcodeimage _returnvalue_2 false)
        ;[1 1 1] Listens for a send from the payout account. This is not guarenteed to happen, so have a timeout or something to go to the next screen.
        (`UserWidget.AddToViewport` (stale `self.Trigger collision.OnComponentBeginOverlap` _returnvalue) 0)
        (`NanoManager.ListenPayoutWaitConfirmation` (`/Game/NanoGameInstance.NanoManager` (stale `self.ReceiveBeginPlay` _asnano_game_instance)) (delegate `OnWalletDrained`) _account (`/Game/NanoGameInstance.NanoWebsocket` (stale `self.ReceiveBeginPlay` _asnano_game_instance)) _expirytime)
        (`KismetSystemLibrary.PrintString` (`KismetStringLibrary.Concat_StrStr` (`KismetStringLibrary.Conv_DoubleToString` _expirytime) " seconds until payment expires"))
        (else
          (`KismetSystemLibrary.PrintString` "private key is empty, pay to play first"))))))

(event `self.ReceiveBeginPlay`
  (bind _asnano_game_instance (cast `/Game/NanoGameInstance` (`GameplayStatics.GetGameInstance`))))

(fn `UserConstructionScript`
  (bind _returnvalue (`PrimitiveComponent.CreateDynamicMaterialInstance` (`self.ButtonMesh`) 2 null "None"))
  (set `self.Button light material` _returnvalue) ; Save a reference to the Dynamic Material Instance for use in the event graph
)