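; BP_AutoReceive is a trigger button that toggles automatic Nano receiving for the local player's seed account (index 0).
; Begin and end overlap share one FlipFlop that switches a dynamic material between green and red.
; A nested FlipFlop on the green step alternates NanoManager Automate and AutomateUnregister over the PlayerState's websocket.
; The send/receive callback is empty, and an older manual websocket registration path is left disconnected.
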(event `OnReceiveData`
  (params (data :type String))
  ;[1 1 1] This is using the websocket stuff manually
  (bind _returnvalue (`WebSocketBlueprintLibrary.JsonToObject` data "/Game/WS_Receive.WS_Receive_C" true))
  (bind _asws_receive (cast `/Game/WS_Receive` _returnvalue))
  (`KismetSystemLibrary.PrintString` (`/Game/WS_Receive.Account` _asws_receive)))

(event `self.Trigger collision.OnComponentBeginOverlap`
  (params (OverlappedComponent :type "PrimitiveComponent Object Reference") (OtherActor :type "Actor Object Reference") (OtherComp :type "PrimitiveComponent Object Reference") (OtherBodyIndex :type Integer) (bFromSweep :type Boolean) (SweepResult :type "HitResult Structure (by ref)"))
  (bind _button_light_material (`self.Button light material`))
  (`/Engine/EditorBlueprintResources/StandardMacros.FlipFlop` :!label _label
    (:`A`
      (`MaterialInstanceDynamic.SetScalarParameterValue` _button_light_material "State" 1.0) ; Change a scalar value in the button material that turns it green
      (`/Engine/EditorBlueprintResources/StandardMacros.FlipFlop`
        (:`A`
          (bind _seed (`/Game/BP_PlayerState.Seed` (stale `self.ReceiveBeginPlay` _asbp_player_state)))
          (bind _returnvalue (`NanoBlueprintLibrary.PrivateKeyFromSeed` _seed))
          (bind _nanomanager (`/Game/BP_PlayerState.NanoManager` (stale `self.ReceiveBeginPlay` _asbp_player_state)))
          (bind _nanowebsocket (`/Game/BP_PlayerState.NanoWebsocket` (stale `self.ReceiveBeginPlay` _asbp_player_state)))
          (`NanoManager.Automate` _nanomanager (delegate `OnSend/Receive`) _returnvalue _nanowebsocket))
        (:`B`
          (bind _returnvalue_2 (`NanoBlueprintLibrary.AccountFromSeed` _seed))
          (`NanoManager.AutomateUnregister` _nanomanager _returnvalue_2 _nanowebsocket))))
    (:`B`
      (`MaterialInstanceDynamic.SetScalarParameterValue` _button_light_material "State" 0.0) ; Change a scalar value in the button material that turns it back to red
    )))

(event `OnSend/Receive`
  (params (data :type "AutomateResponseData Structure")))

(event `self.Trigger collision.OnComponentEndOverlap`
  (params (OverlappedComponent :type "PrimitiveComponent Object Reference") (OtherActor :type "Actor Object Reference") (OtherComp :type "PrimitiveComponent Object Reference") (OtherBodyIndex :type Integer))
  (goto _label))

(event `self.ReceiveBeginPlay`
  (bind _asbp_player_state (cast `/Game/BP_PlayerState` (`Controller.PlayerState` (`GameplayStatics.GetPlayerController` 0)))))

(fn `UserConstructionScript`
  (bind _returnvalue (`PrimitiveComponent.CreateDynamicMaterialInstance` (`self.ButtonMesh`) 2 null "None"))
  (set `self.Button light material` _returnvalue) ; Save a reference to the Dynamic Material Instance for use in the event graph
)