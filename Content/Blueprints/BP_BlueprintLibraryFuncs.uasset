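; Trigger button Blueprint that exercises the Nano Blueprint library functions and prints the results to screen.
; Begin and end overlap share a FlipFlop that alternately turns the button green and runs the tests, or turns it red, via a dynamic material.
; The tests validate and convert hardcoded raw and Nano amounts.
; They then save the game instance's seed to a password-protected, timestamp-named file through NanoManager and verify it reads back.
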(event `self.ReceiveBeginPlay`
  (bind _asnano_game_instance (cast `/Game/NanoGameInstance` (`GameplayStatics.GetGameInstance`))))

(event `self.Trigger collision.OnComponentBeginOverlap`
  (params (OverlappedComponent :type "PrimitiveComponent Object Reference") (OtherActor :type "Actor Object Reference") (OtherComp :type "PrimitiveComponent Object Reference") (OtherBodyIndex :type Integer) (bFromSweep :type Boolean) (SweepResult :type "HitResult Structure (by ref)"))
  (bind _button_light_material (`self.Button light material`))
  (`/Engine/EditorBlueprintResources/StandardMacros.FlipFlop` :!label _label
    (:`A`
      (`MaterialInstanceDynamic.SetScalarParameterValue` _button_light_material "State" 1.0) ; Change a scalar value in the button material that turns it green
      ;[1 1 1] Check raw to Nano
      (bind _output_get (set `self.10^30raw` "1000000000000000000000000000000"))
      (bind _returnvalue (`NanoBlueprintLibrary.ValidateRaw` _output_get))
      (if _returnvalue
        (bind _returnvalue_2 (`NanoBlueprintLibrary.RawToNano` _output_get))
        (`KismetSystemLibrary.PrintString` (`KismetStringLibrary.Concat_StrStr` (`KismetStringLibrary.Concat_StrStr` (`KismetStringLibrary.Concat_StrStr` _output_get " Is ") _returnvalue_2) " Nano"))
        (bind _output_get_2 (set `self.10^29raw` "100000000000000000000000000000"))
        (bind _returnvalue_3 (`NanoBlueprintLibrary.ValidateRaw` _output_get_2))
        (if _returnvalue_3
          (bind _returnvalue_4 (`NanoBlueprintLibrary.RawToNano` _output_get_2))
          (`KismetSystemLibrary.PrintString` (`KismetStringLibrary.Concat_StrStr` (`KismetStringLibrary.Concat_StrStr` (`KismetStringLibrary.Concat_StrStr` _output_get_2 " Is ") _returnvalue_4) " Nano"))
          ;[1 1 1] Check Nano to raw
          (bind _returnvalue_5 (`NanoBlueprintLibrary.NanoToRaw` "1"))
          (`KismetSystemLibrary.PrintString` _returnvalue_5)
          (bind _seed (`/Game/NanoGameInstance.Seed` (stale `self.ReceiveBeginPlay` _asnano_game_instance)))
          ;[1 1 1] Check seeds can be written to filesystem and read correctly
          (if (`KismetStringLibrary.EqualEqual_StrStr` _seed)
            (`KismetSystemLibrary.PrintString` "No seed detected")
            (else
              (bind _output_get_3 (set `self.seedFileName` (`KismetStringLibrary.Concat_StrStr` (`KismetStringLibrary.Conv_IntToString` (`KismetMathLibrary.GetMillisecond` (`KismetMathLibrary.UtcNow`))) ".txt")))
              (bind _nanomanager (`/Game/NanoGameInstance.NanoManager` (stale `self.ReceiveBeginPlay` _asnano_game_instance)))
              (`NanoManager.SaveSeed` _nanomanager _seed _output_get_3 (`self.password`))
              (`KismetSystemLibrary.PrintString` (`KismetStringLibrary.Concat_StrStr` "Saved seed file: " _output_get_3))
              (`KismetSystemLibrary.PrintString` (`KismetStringLibrary.Concat_StrStr` "Num seed files: " (`KismetStringLibrary.Conv_IntToString` (`NanoManager.GetNumSeedFiles` _nanomanager))))
              (bind _returnvalue_6 (`NanoManager.GetPlainSeed` _nanomanager _output_get_3 (`self.password`)))
              (if (and (`KismetStringLibrary.EqualEqual_StrStr` _seed _returnvalue_6) (`KismetStringLibrary.NotEqual_StrStr` _returnvalue_6))
                (`KismetSystemLibrary.PrintString` "Read from seed file succeeded!")
                (else
                  (`KismetSystemLibrary.PrintString` "Read from seed file failed!")))))
          (else
            (`KismetSystemLibrary.PrintString` "Invalid Raw amount" :!label _label_2)))
        (else
          (goto _label_2))))
    (:`B`
      (`MaterialInstanceDynamic.SetScalarParameterValue` _button_light_material "State" 0.0) ; Change a scalar value in the button material that turns it back to red
    )))

(event `self.Trigger collision.OnComponentEndOverlap`
  (params (OverlappedComponent :type "PrimitiveComponent Object Reference") (OtherActor :type "Actor Object Reference") (OtherComp :type "PrimitiveComponent Object Reference") (OtherBodyIndex :type Integer))
  (goto _label))

(fn `UserConstructionScript`
  (bind _returnvalue (`PrimitiveComponent.CreateDynamicMaterialInstance` (`self.ButtonMesh`) 2 null "None"))
  (set `self.Button light material` _returnvalue) ; Save a reference to the Dynamic Material Instance for use in the event graph
)