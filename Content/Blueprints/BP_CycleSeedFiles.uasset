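; Trigger button Blueprint that cycles through saved Nano seed files and shows the selected account on a room display.
; Overlap begin and end share a FlipFlop that toggles the button light and, on activation, decrypts the next seed with a password.
; It derives the account, stores it in the NanoGameInstance and swaps the websocket watch to it.
; A looping timer polls the wallet balance to update balance and pending text.
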(event `self.Trigger collision.OnComponentBeginOverlap`
  (params (OverlappedComponent :type "PrimitiveComponent Object Reference") (OtherActor :type "Actor Object Reference") (OtherComp :type "PrimitiveComponent Object Reference") (OtherBodyIndex :type Integer) (bFromSweep :type Boolean) (SweepResult :type "HitResult Structure (by ref)"))
  (bind _button_light_material (`self.Button light material`))
  (`/Engine/EditorBlueprintResources/StandardMacros.FlipFlop` :!label _label
    (:`A`
      (`MaterialInstanceDynamic.SetScalarParameterValue` _button_light_material "State" 1.0) ; Change a scalar value in the button material that turns it green
      (bind _nanomanager (`/Game/NanoGameInstance.NanoManager` (stale `self.ReceiveBeginPlay` _asnano_game_instance)))
      (bind _nanowebsocket (`/Game/NanoGameInstance.NanoWebsocket` (stale `self.ReceiveBeginPlay` _asnano_game_instance)))
      ;[1 1 1] First do some cleanup if already tracking an account
      (`NanoManager.Unwatch` _nanomanager (`/Game/NanoGameInstance.Account` (stale `self.ReceiveBeginPlay` _asnano_game_instance)) (`self.watchId`) _nanowebsocket)
      (bind _returnvalue (`NanoManager.GetSeedFiles` _nanomanager))
      (bind _returnvalue_2 (`KismetArrayLibrary.Array_Length` _returnvalue))
      (if (== _returnvalue_2 0)
        (`KismetSystemLibrary.PrintString` "Do not have any seed files, create them as Misc blueprint library portal")
        (else
          (if (> (`self.seedFileIndex`) (- _returnvalue_2 1))
            (set `self.seedFileIndex` 0) ; Reset index
          )
          ;[1 1 1] Create seed
          (bind _output_get (set `/Game/NanoGameInstance.Seed` (`NanoManager.GetPlainSeed` _nanomanager (`BlueprintPathsLibrary.GetCleanFilename` (`|GetArrayItem` _returnvalue (`self.seedFileIndex`))) (`self.password`)) (stale `self.ReceiveBeginPlay` _asnano_game_instance)))
          (`/Engine/EditorBlueprintResources/StandardMacros.IncrementInt` (`self.seedFileIndex`)
            (:`  `
              ;[1 1 1] Set text for for generated account
              (bind _returnvalue_3 (`NanoBlueprintLibrary.AccountFromSeed` _output_get))
              (`TextRenderComponent.K2_SetText` (`/Game/Blueprints/Seed_Description.AccountAddressText` (`self.RoomDescription`)) (`KismetTextLibrary.Conv_StringToText` _returnvalue_3))
              (bind _output_get_2 (set `/Game/NanoGameInstance.Account` _returnvalue_3 (stale `self.ReceiveBeginPlay` _asnano_game_instance)))
              ;[1 1 1] Poll With Get Wallet Balance, this is inefficient
              (`KismetSystemLibrary.K2_SetTimer` null "UpdateBalance" 1.0 true)
              ;[1 1 1] This registers this account with the websocket to get confirmation callbacks
              (bind _returnvalue_4 (`NanoManager.Watch` :`self` _nanomanager :`account` _output_get_2 :`websocket` _nanowebsocket))
              (set `self.watchId` _returnvalue_4))))))
    (:`B`
      (`MaterialInstanceDynamic.SetScalarParameterValue` _button_light_material "State" 0.0) ; Change a scalar value in the button material that turns it back to red
    )))

(event `self.Trigger collision.OnComponentEndOverlap`
  (params (OverlappedComponent :type "PrimitiveComponent Object Reference") (OtherActor :type "Actor Object Reference") (OtherComp :type "PrimitiveComponent Object Reference") (OtherBodyIndex :type Integer))
  (goto _label))

(event `UpdateBalance`
  ;[1 1 1] Poll With Get Wallet Balance, this is inefficient
  (bind _account (`/Game/NanoGameInstance.Account` (stale `self.ReceiveBeginPlay` _asnano_game_instance)))
  (if (`KismetStringLibrary.NotEqual_StrStr` _account)
    (`NanoManager.GetWalletBalance` (`/Game/NanoGameInstance.NanoManager` (stale `self.ReceiveBeginPlay` _asnano_game_instance)) (delegate `OnGetBalance`) _account)))

(event `self.ReceiveBeginPlay`
  (bind _asnano_game_instance (cast `/Game/NanoGameInstance` (`GameplayStatics.GetGameInstance`))))

(event `OnGetBalance`
  (params (data :type "GetBalanceResponseData Structure"))
  (bind (_account _balance _pending _error) (break `GetBalanceResponseData` data))
  (bind _roomdescription (`self.RoomDescription`))
  ;[1 1 1] Poll With Get Wallet Balance, this is inefficient
  (if _error
    (`KismetSystemLibrary.PrintString` "GetBalanceFailed")
    (else
      (`TextRenderComponent.K2_SetText` (`/Game/Blueprints/Seed_Description.Balance` _roomdescription) (`KismetTextLibrary.Conv_StringToText` _balance))
      (`TextRenderComponent.K2_SetText` (`/Game/Blueprints/Seed_Description.Pending` _roomdescription) (`KismetTextLibrary.Conv_StringToText` _pending)))))

(fn `UserConstructionScript`
  (bind _returnvalue (`PrimitiveComponent.CreateDynamicMaterialInstance` (`self.ButtonMesh`) 2 null "None"))
  (set `self.Button light material` _returnvalue) ; Save a reference to the Dynamic Material Instance for use in the event graph
)