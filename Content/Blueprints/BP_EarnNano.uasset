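; BP_EarnNano is a trigger button that requests Nano cryptocurrency for the player's account when stepped on.
; Begin and end overlaps share one FlipFlop, alternately turning the button light green while calling the player state's NanoManager, and back to red.
; A callback prints errors or updates the RoomDescription text on receipt.
; The construction script creates the light's dynamic material, and BeginPlay caches the first player's BP_PlayerState.
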(event `self.Trigger collision.OnComponentBeginOverlap`
  (params (OverlappedComponent :type "PrimitiveComponent Object Reference") (OtherActor :type "Actor Object Reference") (OtherComp :type "PrimitiveComponent Object Reference") (OtherBodyIndex :type Integer) (bFromSweep :type Boolean) (SweepResult :type "HitResult Structure (by ref)"))
  (bind _button_light_material (`self.Button light material`))
  (`/Engine/EditorBlueprintResources/StandardMacros.FlipFlop` :!label _label
    (:`A`
      (`MaterialInstanceDynamic.SetScalarParameterValue` _button_light_material "State" 1.0) ; Change a scalar value in the button material that turns it green
      (`NanoManager.RequestNano` (`/Game/BP_PlayerState.NanoManager` (stale `self.ReceiveBeginPlay` _asbp_player_state)) (delegate `OnReceiveNano`) (`/Game/BP_PlayerState.Account` (stale `self.ReceiveBeginPlay` _asbp_player_state))))
    (:`B`
      (`MaterialInstanceDynamic.SetScalarParameterValue` _button_light_material "State" 0.0) ; Change a scalar value in the button material that turns it back to red
    )))

(event `OnReceiveNano`
  (params (data :type "RequestNanoResponseData Structure"))
  (if (`.error` (break `RequestNanoResponseData` data))
    (`KismetSystemLibrary.PrintString` "Error requesting Nano")
    (else
      (bind _output_get (set `self.Text` "Received Nano"))
      (`TextRenderComponent.K2_SetText` (`/Game/Blueprints/Earn_Nano_Description.ReceivedText` (`self.RoomDescription`)) _output_get))))

(event `self.Trigger collision.OnComponentEndOverlap`
  (params (OverlappedComponent :type "PrimitiveComponent Object Reference") (OtherActor :type "Actor Object Reference") (OtherComp :type "PrimitiveComponent Object Reference") (OtherBodyIndex :type Integer))
  (goto _label))

(event `self.ReceiveBeginPlay`
  (bind _asbp_player_state (cast `/Game/BP_PlayerState` (`Controller.PlayerState` (`GameplayStatics.GetPlayerController` 0)))))

(fn `UserConstructionScript`
  (bind _returnvalue (`PrimitiveComponent.CreateDynamicMaterialInstance` (`self.ButtonMesh`) 2 null "None"))
  (set `self.Button light material` _returnvalue) ; Save a reference to the Dynamic Material Instance for use in the event graph
)