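; BP_Handoff is a trigger button that pays Nano cryptocurrency to open a ServerWall door.
; Begin and end overlap share a FlipFlop that toggles the button light via a dynamic material, starting payment on each green toggle.
; MakeSendBlock builds a block for the wall's amount, which BP_PlayerController.OpenDoor hands to the listening server.
; A disabled branch shows the same flow done explicitly through frontier lookup, work generation and manual block creation.
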(event `OnAccountFrontier`
  (params (data :type "AccountFrontierResponseData Structure"))
  (bind (_account _hash _balance _representative _error) (break `AccountFrontierResponseData` data))
  (bind _nanogameinstance (`self.NanoGameInstance`))
  ;[1 1 1] Same as below, but more explicit
  ;;[1 1 1] Get frontier information
  (if _error
    (`KismetSystemLibrary.PrintString` "Error getting the frontier for the account")
    (else
      (set `self.Frontier` _hash)
      (set `self.Representative` _representative)
      ;;[1 1 1] Create the block
      (bind _returnvalue (`NanoBlueprintLibrary.Subtract` _balance (`/Game/Blueprints/ServerWall.Amount` (`self.ServerWall`))))
      (bind _returnvalue_2 (`NanoBlueprintLibrary.PublicKeyFromAccount` (`/Game/NanoGameInstance.PaymentAccount` _nanogameinstance)))
      (`KismetSystemLibrary.PrintString` "Key")
      (bind _returnvalue_3 (`NanoBlueprintLibrary.PrivateKeyFromSeed` (`/Game/NanoGameInstance.Seed` _nanogameinstance)))
      (`NanoManager.WorkGenerate` (`/Game/NanoGameInstance.NanoManager` _nanogameinstance) (delegate `OnWorkGenerate`) _hash))))

(event `OnWorkGenerate`
  (params (data :type "WorkGenerateResponseData Structure"))
  (bind (_hash _work _error) (break `WorkGenerateResponseData` data))
  ;[1 1 1] Same as below, but more explicit
  ;;[1 1 1] Create the block
  (if _error
    (`KismetSystemLibrary.PrintString` "Failed to generate work")
    (else
      (`KismetSystemLibrary.PrintString` "CallOpenDoor")
      (set `self.Block` (make `Block` (`/Game/NanoGameInstance.Account` (`self.NanoGameInstance`)) (`self.Frontier`) (`self.Representative`) (stale `OnAccountFrontier` _returnvalue) (stale `OnAccountFrontier` _returnvalue_2) (stale `OnAccountFrontier` _returnvalue_3) _work))
      ;[1 1 1] Hand it off to the server which is listening for a payment made
      (bind _asbp_player_controller (cast `/Game/BP_PlayerController` (`GameplayStatics.GetPlayerController` 0) :!label _label))
      (`/Game/BP_PlayerController.OpenDoor` _asbp_player_controller (`self.Block`) (`self.ServerWall`)))))

(event `self.Trigger collision.OnComponentBeginOverlap`
  (params (OverlappedComponent :type "PrimitiveComponent Object Reference") (OtherActor :type "Actor Object Reference") (OtherComp :type "PrimitiveComponent Object Reference") (OtherBodyIndex :type Integer) (bFromSweep :type Boolean) (SweepResult :type "HitResult Structure (by ref)"))
  (bind _nanogameinstance (`self.NanoGameInstance`))
  (bind _button_light_material (`self.Button light material`))
  (bind _nanogameinstance_2 (`self.NanoGameInstance`))
  (`/Engine/EditorBlueprintResources/StandardMacros.FlipFlop` :!label _label_2
    (:`A`
      (`MaterialInstanceDynamic.SetScalarParameterValue` _button_light_material "State" 1.0) ; Change a scalar value in the button material that turns it green
      (if false
        ;[1 1 1] Same as below, but more explicit
        ;;[1 1 1] Get frontier information
        (`NanoManager.AccountFrontier` (`/Game/NanoGameInstance.NanoManager` _nanogameinstance) (delegate `OnAccountFrontier`) (`/Game/NanoGameInstance.Account` _nanogameinstance))
        (else
          ;[1 1 1] Create block using utility function (same as above)
          (bind _returnvalue (`NanoBlueprintLibrary.PrivateKeyFromSeed` (`/Game/NanoGameInstance.Seed` _nanogameinstance_2)))
          (`NanoManager.MakeSendBlock` (`/Game/NanoGameInstance.NanoManager` _nanogameinstance_2) (delegate `OnMakeSendBlock`) _returnvalue (`/Game/Blueprints/ServerWall.Amount` (`self.ServerWall`)) (`/Game/NanoGameInstance.PaymentAccount` _nanogameinstance_2)))))
    (:`B`
      (`MaterialInstanceDynamic.SetScalarParameterValue` _button_light_material "State" 0.0) ; Change a scalar value in the button material that turns it back to red
    )))

(event `OnMakeSendBlock`
  (params (data :type "MakeBlockResponseData Structure"))
  (bind (_block _error) (break `MakeBlockResponseData` data))
  ;[1 1 1] Create block using utility function (same as above)
  (if _error
    (`KismetSystemLibrary.PrintString` "Error making send block")
    (else
      (set `self.Block` _block)
      (goto _label))))

(event `self.Trigger collision.OnComponentEndOverlap`
  (params (OverlappedComponent :type "PrimitiveComponent Object Reference") (OtherActor :type "Actor Object Reference") (OtherComp :type "PrimitiveComponent Object Reference") (OtherBodyIndex :type Integer))
  (goto _label_2))

(event `self.ReceiveBeginPlay`
  (bind _asnano_game_instance (cast `/Game/NanoGameInstance` (`GameplayStatics.GetGameInstance`)))
  (set `self.NanoGameInstance` _asnano_game_instance))

(fn `UserConstructionScript`
  (bind _returnvalue (`PrimitiveComponent.CreateDynamicMaterialInstance` (`self.ButtonMesh`) 2 null "None"))
  (set `self.Button light material` _returnvalue) ; Save a reference to the Dynamic Material Instance for use in the event graph
)