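; Demo button that generates a new Nano cryptocurrency account for the player and displays its address and balance.
; Trigger begin and end overlaps share a FlipFlop, alternately lighting the button green while creating an account, and resetting it to red.
; Creation stores seed and account on BP_PlayerState and moves the NanoManager websocket watch to the new account.
; A looping timer polls wallet balance to update RoomDescription's balance and pending text.
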(event `self.Trigger collision.OnComponentBeginOverlap`
  (params (OverlappedComponent :type "PrimitiveComponent Object Reference") (OtherActor :type "Actor Object Reference") (OtherComp :type "PrimitiveComponent Object Reference") (OtherBodyIndex :type Integer) (bFromSweep :type Boolean) (SweepResult :type "HitResult Structure (by ref)"))
  (bind _button_light_material (`self.Button light material`))
  (`/Engine/EditorBlueprintResources/StandardMacros.FlipFlop` :!label _label
    (:`A`
      (`MaterialInstanceDynamic.SetScalarParameterValue` _button_light_material "State" 1.0) ; Change a scalar value in the button material that turns it green
      ;[1 1 1] First do some cleanup if already tracking an account
      (`NanoManager.Unwatch` (`/Game/BP_PlayerState.NanoManager` (stale `self.ReceiveBeginPlay` _asbp_player_state)) (`/Game/BP_PlayerState.Account` (stale `self.ReceiveBeginPlay` _asbp_player_state)) (`self.watchId`) (`/Game/BP_PlayerState.NanoWebsocket` (stale `self.ReceiveBeginPlay` _asbp_player_state)))
      ;[1 1 1] Create seed
      (bind _returnvalue (`NanoBlueprintLibrary.CreateSeed`))
      (bind _output_get (set `/Game/BP_PlayerState.Seed` _returnvalue (stale `self.ReceiveBeginPlay` _asbp_player_state)))
      ;[1 1 1] Set text for for generated account
      (bind _returnvalue_2 (`NanoBlueprintLibrary.AccountFromSeed` _output_get))
      (`TextRenderComponent.K2_SetText` (`/Game/Blueprints/Seed_Description.AccountAddressText` (`self.RoomDescription`)) (`KismetTextLibrary.Conv_StringToText` _returnvalue_2))
      (bind _output_get_2 (set `/Game/BP_PlayerState.Account` _returnvalue_2 (stale `self.ReceiveBeginPlay` _asbp_player_state)))
      ;[1 1 1] This registers this account with the websocket to get confirmation callbacks
      (bind _returnvalue_3 (`NanoManager.Watch` :`self` (`/Game/BP_PlayerState.NanoManager` (stale `self.ReceiveBeginPlay` _asbp_player_state)) :`account` _output_get_2 :`websocket` (`/Game/BP_PlayerState.NanoWebsocket` (stale `self.ReceiveBeginPlay` _asbp_player_state))))
      (set `self.watchId` _returnvalue_3))
    (:`B`
      (`MaterialInstanceDynamic.SetScalarParameterValue` _button_light_material "State" 0.0) ; Change a scalar value in the button material that turns it back to red
    )))

(event `self.Trigger collision.OnComponentEndOverlap`
  (params (OverlappedComponent :type "PrimitiveComponent Object Reference") (OtherActor :type "Actor Object Reference") (OtherComp :type "PrimitiveComponent Object Reference") (OtherBodyIndex :type Integer))
  (goto _label))

(event `self.ReceiveBeginPlay`
  (bind _asbp_player_state (cast `/Game/BP_PlayerState` (`Controller.PlayerState` (`GameplayStatics.GetPlayerController` 0))))
  ;[1 1 1] Poll With Get Wallet Balance, this is inefficient
  (`KismetSystemLibrary.K2_SetTimer` null "UpdateBalance" 2.0 true))

(event `UpdateBalance`
  ;[1 1 1] Poll With Get Wallet Balance, this is inefficient
  (bind _account (`/Game/BP_PlayerState.Account` (stale `self.ReceiveBeginPlay` _asbp_player_state)))
  (if (`KismetStringLibrary.NotEqual_StrStr` _account)
    (`NanoManager.GetWalletBalance` (`/Game/BP_PlayerState.NanoManager` (stale `self.ReceiveBeginPlay` _asbp_player_state)) (delegate `OnGetBalance`) _account)))

(event `OnGetBalance`
  (params (data :type "GetBalanceResponseData Structure"))
  (bind (_account _balance _pending _error) (break `GetBalanceResponseData` data))
  (bind _roomdescription (`self.RoomDescription`))
  ;[1 1 1] Poll With Get Wallet Balance, this is inefficient
  (if _error
    (`KismetSystemLibrary.PrintString` "GetBalanceFailed")
    (else
      (`TextRenderComponent.K2_SetText` (`/Game/Blueprints/Seed_Description.Balance` _roomdescription) (`KismetTextLibrary.Conv_StringToText` _balance))
      (`TextRenderComponent.K2_SetText` (`/Game/Blueprints/Seed_Description.Pending` _roomdescription) (`KismetTextLibrary.Conv_StringToText` _pending)))))

(fn `UserConstructionScript`
  (bind _returnvalue (`PrimitiveComponent.CreateDynamicMaterialInstance` (`self.ButtonMesh`) 2 null "None"))
  (set `self.Button light material` _returnvalue) ; Save a reference to the Dynamic Material Instance for use in the event graph
)