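; Trigger button that displays a Nano payment QR code on screen when overlapped and prints a message once payment arrives.
; Begin and end overlap share a FlipFlop that toggles the button's dynamic material between green and red and adds or removes the QR widget.
; Using the player state's account, it generates a random-amount QR texture, registers with the websocket and awaits confirmation through NanoManager, whose callback removes the widget.
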(event `self.Trigger collision.OnComponentBeginOverlap`
  (params (OverlappedComponent :type "PrimitiveComponent Object Reference") (OtherActor :type "Actor Object Reference") (OtherComp :type "PrimitiveComponent Object Reference") (OtherBodyIndex :type Integer) (bFromSweep :type Boolean) (SweepResult :type "HitResult Structure (by ref)"))
  (bind _button_light_material (`self.Button light material`))
  (bind _returnvalue (`KismetStringLibrary.Conv_IntToString` (`KismetMathLibrary.RandomInteger` 100000)))
  (`/Engine/EditorBlueprintResources/StandardMacros.FlipFlop` :!label _label
    (:`A`
      (`MaterialInstanceDynamic.SetScalarParameterValue` _button_light_material "State" 1.0) ; Change a scalar value in the button material that turns it green
      ;[1 1 1] Show the QR Code
      (bind _returnvalue_2 (`|CreateWidget` "/Game/Blueprints/QRCodePlane.QRCodePlane_C"))
      (bind _account (`/Game/BP_PlayerState.Account` (stale `self.ReceiveBeginPlay` _asbp_player_state)))
      (if (`KismetStringLibrary.NotEqual_StrStr` _account)
        (bind _returnvalue_3 (`NanoBlueprintLibrary.GenerateQRCodeTextureWithAmount` (`self.size_pixels`) _account _returnvalue))
        (`Image.SetBrushFromTexture` (`/Game/Blueprints/QRCodePlane.QRCodeImage` _returnvalue_2) _returnvalue_3 false)
        (`UserWidget.AddToViewport` _returnvalue_2 0)
        (bind _nanowebsocket (`/Game/BP_PlayerState.NanoWebsocket` (stale `self.ReceiveBeginPlay` _asbp_player_state)))
        ;[1 1 1] Register with websocket and listen for payment of this amount to this account
        (`NanoWebsocket.RegisterAccount` _nanowebsocket _account)
        (`NanoManager.ListenForPaymentWaitConfirmation` (`/Game/BP_PlayerState.NanoManager` (stale `self.ReceiveBeginPlay` _asbp_player_state)) (delegate `OnPaymentMade`) _account _returnvalue)
        (else
          (`KismetSystemLibrary.PrintString` "Have not created a seed yet!"))))
    (:`B`
      (`MaterialInstanceDynamic.SetScalarParameterValue` _button_light_material "State" 0.0) ; Change a scalar value in the button material that turns it back to red
      (`Widget.RemoveFromParent` _returnvalue_2)
      (`NanoWebsocket.UnregisterAccount` _nanowebsocket _account))))

(event `self.Trigger collision.OnComponentEndOverlap`
  (params (OverlappedComponent :type "PrimitiveComponent Object Reference") (OtherActor :type "Actor Object Reference") (OtherComp :type "PrimitiveComponent Object Reference") (OtherBodyIndex :type Integer))
  (goto _label))

(event `OnPaymentMade`
  (params (hash :type String))
  ;[1 1 1] Register with websocket and listen for payment of this amount to this account
  (`KismetSystemLibrary.PrintString` "Payment made!")
  (`Widget.RemoveFromParent` (stale `self.Trigger collision.OnComponentBeginOverlap` _returnvalue_2)))

(event `self.ReceiveBeginPlay`
  (bind _asbp_player_state (cast `/Game/BP_PlayerState` (`Controller.PlayerState` (`GameplayStatics.GetPlayerController` 0)))))

(fn `UserConstructionScript`
  (bind _returnvalue (`PrimitiveComponent.CreateDynamicMaterialInstance` (`self.ButtonMesh`) 2 null "None"))
  (set `self.Button light material` _returnvalue) ; Save a reference to the Dynamic Material Instance for use in the event graph
)