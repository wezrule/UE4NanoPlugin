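; Trigger button actor that receives pending Nano cryptocurrency into the game instance's account.
; Overlap begin and end share a FlipFlop that toggles the dynamic material light green or red, querying pending blocks on green.
; Chained NanoManager callbacks then fetch the frontier (zero for new accounts) and balance, add the first pending amount, and process a block signed with the seed-derived key.
; Success updates the RoomDescription text; balance or processing errors print messages.
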(event `OnAccountFrontier`
  (params (data :type "AccountFrontierResponseData Structure"))
  (bind (_account _hash _balance _representative) (break `AccountFrontierResponseData` data))
  ;[1 1 1] Get account frontier
  (bind _returnvalue (`NanoBlueprintLibrary.PublicKeyFromAccount` (`/Game/NanoGameInstance.Account` (stale `self.ReceiveBeginPlay` _asnano_game_instance))))
  (if (`KismetStringLibrary.EqualEqual_StrStr` _hash _returnvalue)
    ;[1 1 1] Previous is 0 for new accounts
    (set `self.Frontier` "0")
    (else
      (set `self.Frontier` _hash)))
  ;[1 1 1] Get Balance
  (`NanoManager.GetWalletBalance` (`/Game/NanoGameInstance.NanoManager` (stale `self.ReceiveBeginPlay` _asnano_game_instance)) (delegate `OnGetWalletBalance`) (`/Game/NanoGameInstance.Account` (stale `self.ReceiveBeginPlay` _asnano_game_instance))))

(event `self.Trigger collision.OnComponentBeginOverlap`
  (params (OverlappedComponent :type "PrimitiveComponent Object Reference") (OtherActor :type "Actor Object Reference") (OtherComp :type "PrimitiveComponent Object Reference") (OtherBodyIndex :type Integer) (bFromSweep :type Boolean) (SweepResult :type "HitResult Structure (by ref)"))
  (bind _button_light_material (`self.Button light material`))
  (`/Engine/EditorBlueprintResources/StandardMacros.FlipFlop` :!label _label
    (:`A`
      (`MaterialInstanceDynamic.SetScalarParameterValue` _button_light_material "State" 1.0) ; Change a scalar value in the button material that turns it green
      (`NanoManager.Pending` (`/Game/NanoGameInstance.NanoManager` (stale `self.ReceiveBeginPlay` _asnano_game_instance)) (delegate `OnPending`) (`/Game/NanoGameInstance.Account` (stale `self.ReceiveBeginPlay` _asnano_game_instance))))
    (:`B`
      (`MaterialInstanceDynamic.SetScalarParameterValue` _button_light_material "State" 0.0) ; Change a scalar value in the button material that turns it back to red
    )))

(event `OnGetWalletBalance`
  (params (data :type "GetBalanceResponseData Structure"))
  (bind (_account _balance _pending _error) (break `GetBalanceResponseData` data))
  ;[1 1 1] Get Balance
  (if _error
    (`KismetSystemLibrary.PrintString` "Error getting balance")
    (else
      (bind (_hash _amount) (break `PendingBlock` (`|GetArrayItem` (`.blocks` (break `PendingResponseData` (stale `OnPending` data))))))
      (bind _returnvalue (`NanoBlueprintLibrary.Add` _balance _amount))
      (bind _returnvalue_2 (`NanoBlueprintLibrary.PrivateKeyFromSeed` (`/Game/NanoGameInstance.Seed` (stale `self.ReceiveBeginPlay` _asnano_game_instance))))
      ;[1 1 1] Process the block
      (`NanoManager.Process` (`/Game/NanoGameInstance.NanoManager` (stale `self.ReceiveBeginPlay` _asnano_game_instance)) (delegate `OnProcess`) (make `Block` (`/Game/NanoGameInstance.Account` (stale `self.ReceiveBeginPlay` _asnano_game_instance)) (`self.Frontier`) (`.representative` (break `AccountFrontierResponseData` (stale `OnAccountFrontier` data))) _returnvalue _hash _returnvalue_2 (`/Game/NanoGameInstance.LastWork` (stale `self.ReceiveBeginPlay` _asnano_game_instance)))))))

(event `self.Trigger collision.OnComponentEndOverlap`
  (params (OverlappedComponent :type "PrimitiveComponent Object Reference") (OtherActor :type "Actor Object Reference") (OtherComp :type "PrimitiveComponent Object Reference") (OtherBodyIndex :type Integer))
  (goto _label))

(event `OnPending`
  (params (data :type "PendingResponseData Structure"))
  (`/Engine/EditorBlueprintResources/StandardMacros.CompareInt` (`KismetArrayLibrary.Array_Length` (`.blocks` (break `PendingResponseData` data)))
    (:`>`
      ;[1 1 1] Get account frontier
      (`NanoManager.AccountFrontier` (`/Game/NanoGameInstance.NanoManager` (stale `self.ReceiveBeginPlay` _asnano_game_instance)) (delegate `OnAccountFrontier`) (`/Game/NanoGameInstance.Account` (stale `self.ReceiveBeginPlay` _asnano_game_instance))))))

(event `OnProcess`
  (params (data :type "ProcessResponseData Structure"))
  ;[1 1 1] Process the block
  (if (`.error` (break `ProcessResponseData` data))
    (`KismetSystemLibrary.PrintString` "Processing block failed")
    (else
      (`TextRenderComponent.K2_SetText` (`/Game/Blueprints/Receive_Description.ReceiveText` (`self.RoomDescription`)) "Block confirmed"))))

(event `self.ReceiveBeginPlay`
  (bind _asnano_game_instance (cast `/Game/NanoGameInstance` (`GameplayStatics.GetGameInstance`))))

(fn `UserConstructionScript`
  (bind _returnvalue (`PrimitiveComponent.CreateDynamicMaterialInstance` (`self.ButtonMesh`) 2 null "None"))
  (set `self.Button light material` _returnvalue) ; Save a reference to the Dynamic Material Instance for use in the event graph
)