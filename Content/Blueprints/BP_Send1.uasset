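; BP_Send1 is a trigger button that sends a small fixed amount of Nano cryptocurrency from the player's account to the RoomDescription account.
; Begin and end overlap share a FlipFlop, alternately turning the button green while requesting the account frontier and turning it red.
; The frontier callback builds a block with the reduced balance and submits it through the player state's NanoManager.
; A looping timer shows the receiver's pending balance on the UFO text.
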(event `OnAccountFrontier`
  (params (data :type "AccountFrontierResponseData Structure"))
  (bind (_account _hash _balance _representative _error) (break `AccountFrontierResponseData` data))
  (bind _bp_playerstate (`self.BP_PlayerState`))
  ;[1 1 1] Get frontier information
  (if _error
    (`KismetSystemLibrary.PrintString` "Error getting the frontier for the account")
    (else
      (set `self.Frontier` _hash)
      (set `self.Representative` _representative)
      ;[1 1 1] Process the send
      (bind _returnvalue (`NanoBlueprintLibrary.Subtract` _balance "5000"))
      (bind _returnvalue_2 (`NanoBlueprintLibrary.PublicKeyFromAccount` (`/Game/Blueprints/Send_Description.Account` (`self.Room Description`))))
      (bind _returnvalue_3 (`NanoBlueprintLibrary.PrivateKeyFromSeed` (`/Game/BP_PlayerState.Seed` _bp_playerstate)))
      (`NanoManager.Process` (`/Game/BP_PlayerState.NanoManager` _bp_playerstate) (delegate `OnProcess`) (make `Block` (`/Game/BP_PlayerState.Account` _bp_playerstate) (`self.Frontier`) (`self.Representative`) _returnvalue _returnvalue_2 _returnvalue_3 (`/Game/BP_PlayerState.LastWork` _bp_playerstate))))))

(event `self.Trigger collision.OnComponentBeginOverlap`
  (params (OverlappedComponent :type "PrimitiveComponent Object Reference") (OtherActor :type "Actor Object Reference") (OtherComp :type "PrimitiveComponent Object Reference") (OtherBodyIndex :type Integer) (bFromSweep :type Boolean) (SweepResult :type "HitResult Structure (by ref)"))
  (bind _bp_playerstate (`self.BP_PlayerState`))
  (bind _button_light_material (`self.Button light material`))
  (`/Engine/EditorBlueprintResources/StandardMacros.FlipFlop` :!label _label
    (:`A`
      (`MaterialInstanceDynamic.SetScalarParameterValue` _button_light_material "State" 1.0) ; Change a scalar value in the button material that turns it green
      ;[1 1 1] Get frontier information
      (`NanoManager.AccountFrontier` (`/Game/BP_PlayerState.NanoManager` _bp_playerstate) (delegate `OnAccountFrontier`) (`/Game/BP_PlayerState.Account` _bp_playerstate)))
    (:`B`
      (`MaterialInstanceDynamic.SetScalarParameterValue` _button_light_material "State" 0.0) ; Change a scalar value in the button material that turns it back to red
    )))

(event `self.Trigger collision.OnComponentEndOverlap`
  (params (OverlappedComponent :type "PrimitiveComponent Object Reference") (OtherActor :type "Actor Object Reference") (OtherComp :type "PrimitiveComponent Object Reference") (OtherBodyIndex :type Integer))
  (goto _label))

(event `OnProcess`
  (params (data :type "ProcessResponseData Structure"))
  ;[1 1 1] Process the send
  (if (`.error` (break `ProcessResponseData` data))
    (`KismetSystemLibrary.PrintString` "Failed to send")
    (else
      (`KismetSystemLibrary.PrintString` "Sent"))))

(event `self.ReceiveBeginPlay`
  (bind _asbp_player_state (cast `/Game/BP_PlayerState` (`Controller.PlayerState` (`GameplayStatics.GetPlayerController` 0))))
  (set `self.BP_PlayerState` _asbp_player_state)
  ;[1 1 1] Poll balance and update text for receiver
  (`KismetSystemLibrary.K2_SetTimer` null "UpdateReceiverBalance" 2.0 true))

(event `UpdateReceiverBalance`
  (bind _account (`/Game/Blueprints/Send_Description.Account` (`self.Room Description`)))
  ;[1 1 1] Poll balance and update text for receiver
  (if (`KismetStringLibrary.NotEqual_StrStr` _account)
    (`NanoManager.GetWalletBalance` (`/Game/BP_PlayerState.NanoManager` (stale `self.ReceiveBeginPlay` _asbp_player_state)) (delegate `OnGetWalletBalance`) _account)))

(event `OnGetWalletBalance`
  (params (data :type "GetBalanceResponseData Structure"))
  (bind (_account _balance _pending _error) (break `GetBalanceResponseData` data))
  ;[1 1 1] Poll balance and update text for receiver
  (if _error
    (`KismetSystemLibrary.PrintString` "Failed to get wallet balance")
    (else
      (`TextRenderComponent.K2_SetText` (`/Game/Blueprints/BP_UFO.BalanceText` (`self.UFO`)) (`KismetTextLibrary.Conv_StringToText` _pending)))))

(fn `UserConstructionScript`
  (bind _returnvalue (`PrimitiveComponent.CreateDynamicMaterialInstance` (`self.ButtonMesh`) 2 null "None"))
  (set `self.Button light material` _returnvalue) ; Save a reference to the Dynamic Material Instance for use in the event graph
)