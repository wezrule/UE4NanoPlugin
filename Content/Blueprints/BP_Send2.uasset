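; BP_Send2 is a trigger button that sends a fixed amount of Nano cryptocurrency from the player's account to the room's account.
; Begin and end overlap share a FlipFlop, alternately turning the button's dynamic material green and starting a send, or turning it red.
; The send fetches the account frontier, checks balance, then submits a block signed with the seed-derived key and awaits confirmation, printing the outcome.
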(event `OnAccountFrontier`
  (params (data :type "AccountFrontierResponseData Structure"))
  (bind (_account _hash _balance _representative _error) (break `AccountFrontierResponseData` data))
  (bind _nanogameinstance (`self.NanoGameInstance`))
  ;[1 1 1] Get frontier information
  (if _error
    (`KismetSystemLibrary.PrintString` "Error getting the frontier for the account")
    (else
      (set `self.Frontier` _hash)
      (set `self.Representative` _representative)
      (bind _returnvalue (`NanoBlueprintLibrary.GreaterOrEqual` _balance "5000"))
      ;[1 1 1] Process the send
      (if _returnvalue
        (bind _returnvalue_2 (`NanoBlueprintLibrary.Subtract` _balance "5000"))
        (bind _returnvalue_3 (`NanoBlueprintLibrary.PublicKeyFromAccount` (`/Game/Blueprints/Send_Description.Account` (`self.Room Description`))))
        (bind _returnvalue_4 (`NanoBlueprintLibrary.PrivateKeyFromSeed` (`/Game/NanoGameInstance.Seed` _nanogameinstance)))
        (`NanoManager.ProcessSendWaitConfirmation` (`/Game/NanoGameInstance.NanoManager` _nanogameinstance) (delegate `OnProcess`) (make `Block` (`/Game/NanoGameInstance.Account` _nanogameinstance) (`self.Frontier`) (`self.Representative`) _returnvalue_2 _returnvalue_3 _returnvalue_4 (`/Game/NanoGameInstance.LastWork` _nanogameinstance)))
        (else
          (`KismetSystemLibrary.PrintString` "Not enough balance"))))))

(event `self.Trigger collision.OnComponentBeginOverlap`
  (params (OverlappedComponent :type "PrimitiveComponent Object Reference") (OtherActor :type "Actor Object Reference") (OtherComp :type "PrimitiveComponent Object Reference") (OtherBodyIndex :type Integer) (bFromSweep :type Boolean) (SweepResult :type "HitResult Structure (by ref)"))
  (bind _nanogameinstance (`self.NanoGameInstance`))
  (bind _button_light_material (`self.Button light material`))
  (bind _account (`/Game/NanoGameInstance.Account` _nanogameinstance))
  (`/Engine/EditorBlueprintResources/StandardMacros.FlipFlop` :!label _label
    (:`A`
      (`MaterialInstanceDynamic.SetScalarParameterValue` _button_light_material "State" 1.0) ; Change a scalar value in the button material that turns it green
      (if (`KismetStringLibrary.NotEqual_StrStr` _account)
        ;[1 1 1] Get frontier information
        (`NanoManager.AccountFrontier` (`/Game/NanoGameInstance.NanoManager` _nanogameinstance) (delegate `OnAccountFrontier`) _account)
        (else
          (`KismetSystemLibrary.PrintString` "No seed detected"))))
    (:`B`
      (`MaterialInstanceDynamic.SetScalarParameterValue` _button_light_material "State" 0.0) ; Change a scalar value in the button material that turns it back to red
    )))

(event `self.Trigger collision.OnComponentEndOverlap`
  (params (OverlappedComponent :type "PrimitiveComponent Object Reference") (OtherActor :type "Actor Object Reference") (OtherComp :type "PrimitiveComponent Object Reference") (OtherBodyIndex :type Integer))
  (goto _label))

(event `self.ReceiveBeginPlay`
  (bind _asnano_game_instance (cast `/Game/NanoGameInstance` (`GameplayStatics.GetGameInstance`)))
  (set `self.NanoGameInstance` _asnano_game_instance))

(event `OnProcess`
  (params (data :type "ProcessResponseData Structure"))
  ;[1 1 1] Process the send
  (if (`.error` (break `ProcessResponseData` data))
    (`KismetSystemLibrary.PrintString` "Failed to send")
    (else
      (`KismetSystemLibrary.PrintString` "Sent"))))

(fn `UserConstructionScript`
  (bind _returnvalue (`PrimitiveComponent.CreateDynamicMaterialInstance` (`self.ButtonMesh`) 2 null "None"))
  (set `self.Button light material` _returnvalue) ; Save a reference to the Dynamic Material Instance for use in the event graph
)