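; Demo button for the Nano cryptocurrency plugin that watches an account and sends it funds when a pawn steps on its trigger.
; Begin and end overlap share a FlipFlop that turns the button's dynamic material green, then red.
; A nested FlipFlop alternates green presses between watching the RoomDescription account while sending a fixed amount from the game instance seed, and unwatching it.
; Websocket callbacks write the received amount to the UFO balance text.
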(event `OnSend/Receive`
  (params (data :type "AutomateResponseData Structure"))
  (bind (_type _account _amount _balance _hash _frontier _representative _error) (break `AutomateResponseData` data))
  ;[1 1 1] Received from websocket
  (if _error
    (`KismetSystemLibrary.PrintString` "Websocket receive failure")
    (else
      (`TextRenderComponent.K2_SetText` (`/Game/Blueprints/BP_UFO.BalanceText` (`self.UFO`)) (`KismetTextLibrary.Conv_StringToText` _amount)))))

(event `self.Trigger collision.OnComponentBeginOverlap`
  (params (OverlappedComponent :type "PrimitiveComponent Object Reference") (OtherActor :type "Actor Object Reference") (OtherComp :type "PrimitiveComponent Object Reference") (OtherBodyIndex :type Integer) (bFromSweep :type Boolean) (SweepResult :type "HitResult Structure (by ref)"))
  (bind _button_light_material (`self.Button light material`))
  (bind _account (`/Game/Blueprints/AutoWatcher.Account` (`self.RoomDescription`)))
  (`/Engine/EditorBlueprintResources/StandardMacros.FlipFlop` :!label _label
    (:`A`
      (`MaterialInstanceDynamic.SetScalarParameterValue` _button_light_material "State" 1.0) ; Change a scalar value in the button material that turns it green
      (`/Engine/EditorBlueprintResources/StandardMacros.FlipFlop`
        (:`A`
          (bind _nanomanager (`/Game/NanoGameInstance.NanoManager` (stale `self.ReceiveBeginPlay` _asnano_game_instance)))
          (bind _nanowebsocket (`/Game/NanoGameInstance.NanoWebsocket` (stale `self.ReceiveBeginPlay` _asnano_game_instance)))
          (bind _returnvalue (`NanoManager.Watch` _nanomanager (delegate `OnSend/Receive`) _account _nanowebsocket))
          (set `self.watcherId` _returnvalue)
          ;[1 1 1] Send
          (bind _returnvalue_2 (`NanoBlueprintLibrary.PrivateKeyFromSeed` (`/Game/NanoGameInstance.Seed` (stale `self.ReceiveBeginPlay` _asnano_game_instance))))
          (`NanoManager.Send` _nanomanager (delegate `OnSend`) _returnvalue_2 _account "100"))
        (:`B`
          (`NanoManager.Unwatch` _nanomanager _account (`self.watcherId`) _nanowebsocket))))
    (:`B`
      (`MaterialInstanceDynamic.SetScalarParameterValue` _button_light_material "State" 0.0) ; Change a scalar value in the button material that turns it back to red
    )))

(event `OnSend`
  (params (data :type "ProcessResponseData Structure"))
  (bind (_hash _error) (break `ProcessResponseData` data))
  ;[1 1 1] Send
  (if _error
    (`KismetSystemLibrary.PrintString` "Send failed")
    (else
      (`KismetSystemLibrary.PrintString` _hash))))

(event `self.Trigger collision.OnComponentEndOverlap`
  (params (OverlappedComponent :type "PrimitiveComponent Object Reference") (OtherActor :type "Actor Object Reference") (OtherComp :type "PrimitiveComponent Object Reference") (OtherBodyIndex :type Integer))
  (goto _label))

(event `self.ReceiveBeginPlay`
  (bind _asnano_game_instance (cast `/Game/NanoGameInstance` (`GameplayStatics.GetGameInstance`))))

(fn `UserConstructionScript`
  (bind _returnvalue (`PrimitiveComponent.CreateDynamicMaterialInstance` (`self.ButtonMesh`) 2 null "None"))
  (set `self.Button light material` _returnvalue) ; Save a reference to the Dynamic Material Instance for use in the event graph
)