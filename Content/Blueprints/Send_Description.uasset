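; Display stand actor that shows a freshly generated crypto account address as its send address.
; On BeginPlay it creates a new seed, derives the account at index zero, stores it and writes it to the SendAddress text.
; The construction script creates dynamic material instances on the base and flat wall meshes and tints both with StandColor.
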(event `self.ReceiveBeginPlay`
  (bind _returnvalue (`NanoBlueprintLibrary.CreateSeed`))
  (bind _returnvalue_2 (`NanoBlueprintLibrary.AccountFromSeed` _returnvalue))
  (bind _output_get (set `self.Account` _returnvalue_2))
  (`TextRenderComponent.K2_SetText` (`self.SendAddress`) (`KismetTextLibrary.Conv_StringToText` _output_get)))

(fn `UserConstructionScript`
  (bind _returnvalue (`PrimitiveComponent.CreateDynamicMaterialInstance` (`self.SM_Base`) 3 null "None"))
  (`MaterialInstanceDynamic.SetVectorParameterValue` _returnvalue "Color" (`self.StandColor`))
  (bind _returnvalue_2 (`PrimitiveComponent.CreateDynamicMaterialInstance` (`self.SM_Base_FlatWall`) 0 null "None"))
  (`MaterialInstanceDynamic.SetVectorParameterValue` _returnvalue_2 "Color" (`self.StandColor`)))